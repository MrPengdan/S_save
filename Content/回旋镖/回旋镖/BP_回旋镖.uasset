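; Boomerang weapon actor that flies from its owner's hand socket toward a target and reattaches afterward.
; 发射 plays a timeline that lerps from the Tick-updated socket position, adding a distance-scaled sideways arc and spin, at double speed for short throws.
; When the timeline finishes, it plays a catch montage and snaps back to the socket.
; Box overlaps with anything but the owner activate a child destruction-field actor.
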(event `self.ReceiveTick`
  (params (DeltaSeconds :type "Float (single-precision)"))
  (set `self.发射点位置` (`SceneComponent.GetSocketLocation` (`Character.Mesh` (`self.拥有者`)) "右手回旋镖")))

(event `发射`
  (params (`目标点位置` :type "Vector Structure"))
  (bind _returnvalue (- (`self.目标点位置`) (`self.发射点位置`)))
  (bind _mesh (`Character.Mesh` (`self.拥有者`)))
  (bind _returnvalue_2 (`KismetMathLibrary.VSize` _returnvalue))
  (set `self.目标点位置` `目标点位置`)
  (`TimelineComponent.SetPlayRate` (`self.发射轨迹时间轴`) (select `bool` (< _returnvalue_2 1000.0) :`false` 1.0 :`true` 2.0 :!type "Float (single-precision)"))
  ;[1 1 1] 设置旋转对要速度
  (`self.K2_SetActorRotation` (`KismetMathLibrary.Conv_VectorToRotator` (* _returnvalue -1.0)))
  (set `self.飞行` true)
  (bind (_direction `_位置` `_新建轨道_2`) (`Timeline|发射轨迹时间轴` :!via `PlayFromStart`)
    (:`Update`
      (`self.K2_SetActorLocation` (+ (`KismetMathLibrary.VLerp` (`self.发射点位置`) (`self.目标点位置`) `_位置`) (* (`KismetMathLibrary.Normal` (`KismetMathLibrary.Cross_VectorVector` (- (`self.发射点位置`) (`self.目标点位置`)) (0.0 0.0 1.0))) `_新建轨道_2` (/ _returnvalue_2 10.0) 3.0)))
      (`self.K2_AddActorLocalRotation` (`KismetMathLibrary.RLerp` (struct) (struct :`Yaw` 1.0) `_位置`)))
    (:`Finished`
      (set `self.飞行` false)
      (`|PlayMontage` _mesh "/Game/回旋镖/动画/飞斧_接斧头1_Montage.飞斧_接斧头1_Montage"
        (:`then`
          (`self.K2_AttachToComponent` _mesh "右手回旋镖" "SnapToTarget" "SnapToTarget" "SnapToTarget"))))))

(event `self.Box.OnComponentBeginOverlap`
  (params (OverlappedComponent :type "PrimitiveComponent Object Reference") (OtherActor :type "Actor Object Reference") (OtherComp :type "PrimitiveComponent Object Reference") (OtherBodyIndex :type Integer) (bFromSweep :type Boolean) (SweepResult :type "HitResult Structure (by ref)"))
  (if (!= OtherActor (`self.拥有者`))
    (`/Game/chaoS破碎/破碎场+旋转.激活` (cast `/Game/chaoS破碎/破碎场+旋转` (`ChildActorComponent.ChildActor` (`self.破碎场+旋转`)) :!pure true))))

(fn `UserConstructionScript`)