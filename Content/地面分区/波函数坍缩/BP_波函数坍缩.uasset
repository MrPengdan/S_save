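; Grid actor for "wave function collapse" terrain that spawns tile meshes at requested positions, fitting each to its neighbors.
; JK生成激活顶点的网格体 converts the position to an actor offset, fires Niagara there and adds a static mesh.
; 计算六个点 searches stored points for six axis neighbors, clearing facing characters in both tiles' six-character "bit" strings.
; Each string is a DT_网格数据表 row name supplying mesh and yaw, so existing neighbors re-tile too.
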(event `新建静态网格组件`
  (params (`相对位置` :type "Vector Structure"))
  (bind _niagara (`self.Niagara`))
  (`SceneComponent.K2_SetRelativeLocation` _niagara `相对位置` false false)
  (`ActorComponent.Activate` _niagara true)
  (bind _returnvalue (`AddComponent|NODE_AddStaticMeshComponent-0` :`RelativeTransform` (`KismetMathLibrary.MakeTransform` `相对位置` (struct) (0.5 0.5 0.5))))
  (set `self.组合的字符串 1` "111111")
  (bind `_自身bit值` (`self.计算六个点` `相对位置` 100.0))
  (`self.根据BIT值更新mesh` `_自身bit值` _returnvalue)
  (`KismetArrayLibrary.Array_AddUnique` (`self.激活点的集合`) (make `/Game/地面分区/波函数坍缩/ST_激活组件信息` `相对位置` _returnvalue `_自身bit值`)))

(event `/Game/地面分区/波函数坍缩/JK_波函数坍塌.JK_生成激活顶点的网格体`
  (params (`位置` :type "Vector Structure"))
  (`self.新建静态网格组件` (- `位置` (`self.K2_GetActorLocation`))))

(fn `UserConstructionScript`
  (`self.计算六个点` (0.0 0.0 0.0)))

(fn `修改组合字符串`
  (params (`拆分的BIT值` :type String) (`要修改的Index` :type Integer) (`要修改的值` :type String :default "1"))
  (returns (`组合的字符串1` :type String))
  (locals (`拆分的数组` :type "Array of String") (`组合的字符串` :type String))
  (bind _output_get (set `local.拆分的数组` (`KismetStringLibrary.GetCharacterArrayFromString` `拆分的BIT值`)))
  (`KismetArrayLibrary.Array_Set` _output_get (- `要修改的Index` 1) `要修改的值`)
  (for _array_element (`local.拆分的数组`)
    (set `local.组合的字符串` (`KismetStringLibrary.Concat_StrStr` (`local.组合的字符串`) _array_element)))
  (return (`local.组合的字符串`)))

(fn `对比位置修改BIT值`
  (params (InputPin :type "Vector Structure") (`要修改的Index` :type Integer) (`要修改的值` :type String) (`自身BIT值` :type String))
  (for (_array_element _array_index) (`self.激活点的集合`)
    (bind (`_点位置` `_静态网格体组件` `_激活的值`) (break `/Game/地面分区/波函数坍缩/ST_激活组件信息` _array_element))
    (if (== `_点位置` InputPin)
      (bind `_组合的字符串1` (`self.修改组合字符串` `_激活的值` `要修改的Index` `要修改的值`))
      (`KismetArrayLibrary.Array_Set` (`self.激活点的集合`) _array_index (make `/Game/地面分区/波函数坍缩/ST_激活组件信息` InputPin `_静态网格体组件` `_组合的字符串1`))
      (`self.根据BIT值更新mesh` `_组合的字符串1` `_静态网格体组件`)
      (set `self.组合的字符串 1` (`self.修改组合字符串` `自身BIT值` (select `int` `要修改的Index` :`0` 0 :`1` 3 :`2` 4 :`3` 1 :`4` 2 :`5` 6 :`6` 5) "0")))))

(fn `根据BIT值更新mesh`
  (params (`BIT值` :type String) (`静态网格组件` :type "StaticMeshComponent Object Reference"))
  (bind _returnvalue (`|GetDataTableRow` "/Game/地面分区/波函数坍缩/DT_网格数据表.DT_网格数据表" (`KismetStringLibrary.Conv_StringToName` `BIT值`))
    (:`then`
      (bind (`_旋转` `_旋转度数` _mesh) (break `/Game/地面分区/波函数坍缩/ST_DT_mash` _returnvalue))
      (`/Engine/EditorBlueprintResources/StandardMacros.IsValid` _mesh
        (:`Is Valid`
          (bind _returnvalue_2 (`StaticMeshComponent.SetStaticMesh` `静态网格组件` _mesh))
          (if _returnvalue_2
            (`SceneComponent.K2_SetRelativeRotation` `静态网格组件` (`KismetMathLibrary.MakeRotator` 0.0 0.0 `_旋转度数`) false false)
            (else
              (`KismetSystemLibrary.PrintString` (`KismetStringLibrary.Concat_StrStr` "无效······" "-" `BIT值`) true true (struct :`G` 0.66 :`B` 1.0 :`A` 1.0) 5.0))))))))

(fn `计算六个点`
  (params (`要查的自身组件` :type "Vector Structure") (`间距1` :type "Float (double-precision)"))
  (returns (`自身BIT值` :type String))
  (locals (`本地点` :type "Vector Structure") (`间距` :type "Float (double-precision)" :default 100.0))
  (bind _x (.x `要查的自身组件`))
  (bind _y (.y `要查的自身组件`))
  (bind _z (.z `要查的自身组件`))
  (bind `_间距` (`local.间距`))
  (set `local.间距` `间距1`)
  (`|ExecutionSequence`
    (:`then_0`
      (bind _output_get (set `local.本地点` (`KismetMathLibrary.MakeVector` (- _x `_间距`) _y _z)))
      (`self.对比位置修改BIT值` _output_get 3 "0" (`self.组合的字符串 1`)))
    (:`then_1`
      (bind _output_get_2 (set `local.本地点` (`KismetMathLibrary.MakeVector` _x (+ _y `_间距`) _z)))
      (`self.对比位置修改BIT值` _output_get_2 2 "0" (`self.组合的字符串 1`)))
    (:`then_2`
      (bind _output_get_3 (set `local.本地点` (`KismetMathLibrary.MakeVector` (+ _x `_间距`) _y _z)))
      (`self.对比位置修改BIT值` _output_get_3 1 "0" (`self.组合的字符串 1`)))
    (:`then_3`
      (bind _output_get_4 (set `local.本地点` (`KismetMathLibrary.MakeVector` _x (- _y `_间距`) _z)))
      (`self.对比位置修改BIT值` _output_get_4 4 "0" (`self.组合的字符串 1`)))
    (:`then_4`
      (bind _output_get_5 (set `local.本地点` (`KismetMathLibrary.MakeVector` _x _y (+ _z `_间距`))))
      (`self.对比位置修改BIT值` _output_get_5 6 "0" (`self.组合的字符串 1`)))
    (:`then_5`
      (bind _output_get_6 (set `local.本地点` (`KismetMathLibrary.MakeVector` _x _y (- _z `_间距`))))
      (`self.对比位置修改BIT值` _output_get_6 5 "0" (`self.组合的字符串 1`)))
    (:`then_6`
      (return (`self.组合的字符串 1`)))))